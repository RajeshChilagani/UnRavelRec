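; Moving platform Blueprint that slides its Floor component back and forth along the world axes enabled by the X, Y and Z flags.
; Each Tick it builds a frame-time-scaled step from Speed and InitalDistance, accumulates it into Distance, and moves Floor without sweep.
; InitalDistance starts as DistanceToMove and flips sign at the travel limits, so it sets direction and also scales velocity with travel distance.
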(event EventBeginPlay
  (Variables|Default|SetInitalDistance (Variables|Default|GetDistanceToMove)))

(event Collision|EventActorBeginOverlap
  (params (OtherActor :type Actor%20Object%20Reference)))

(event EventTick
  (params (DeltaSeconds :type Float%20%28single-precision%29))
  (bind _floor (Variables|Default|Getfloor))
  (bind _floor_2 (Variables|Default|Getfloor))
  (bind _floor_3 (Variables|Default|Getfloor))
  (bind _returnvalue (Transformation|GetWorldLocation _floor_3))
  (bind _returnvalue_2 (Transformation|GetWorldLocation _floor))
  (bind _returnvalue_3 (Transformation|GetWorldLocation _floor_2))
  (Variables|Default|SetDelta (* (* (Variables|Default|GetSpeed) (Utilities|Time|GetWorldDeltaSeconds)) (Variables|Default|GetInitalDistance)))
  (Variables|Default|SetDistance (+ (Variables|Default|GetDistance) (Variables|Default|GetDelta)))
  (Utilities|FlowControl|Sequence
    (:then_0
      (if (Variables|Default|GetX)
        (Variables|Default|SetTemp (Math|Vector|MakeVector (+ (Variables|Default|GetDelta) (.x _returnvalue)) (.y _returnvalue) (.z _returnvalue)))
        (Transformation|SetWorldLocation (Variables|Default|Getfloor) (Variables|Default|GetTemp) false false :!label _label)
        (Utilities|FlowControl|Sequence
          (:then_0
            (if (>= (Variables|Default|GetDistance) (Math|Float|Absolute(Float) (Variables|Default|GetDistanceToMove)))
              (Variables|Default|SetInitalDistance (* -1.0 (Variables|Default|GetDistanceToMove)))))
          (:then_1
            (if (<= (Variables|Default|GetDistance) 0.0)
              (Variables|Default|SetInitalDistance (* (Variables|Default|GetDistanceToMove) 1.0)))))))
    (:then_1
      (if (Variables|Default|GetY)
        (Variables|Default|SetTemp (Math|Vector|MakeVector (.x _returnvalue_2) (+ (Variables|Default|GetDelta) (.y _returnvalue_2)) (.z _returnvalue_2)))
        (goto _label)))
    (:then_2
      (if (Variables|Default|GetZ)
        (Variables|Default|SetTemp (Math|Vector|MakeVector (.x _returnvalue_3) (.y _returnvalue_3) (+ (Variables|Default|GetDelta) (.z _returnvalue_3))))
        (goto _label)))))

(fn ConstructionScript)