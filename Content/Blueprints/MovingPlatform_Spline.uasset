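; A side-scroller moving platform that travels along a spline while the player character is inside its trigger box and returns toward the start once the character leaves.
; Box overlap events toggle forward and reverse flags, which Tick reads to call MoveOnSpline with positive or negated Speed.
; MoveOnSpline advances a stored distance using delta time, places the Cube at that spline point, and clears the matching flag near either end.
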(event OnComponentBeginOverlap(Box)
  (params (OverlappedComponent :type Primitive%20Component%20Object%20Reference) (OtherActor :type Actor%20Object%20Reference) (OtherComp :type Primitive%20Component%20Object%20Reference) (OtherBodyIndex :type Integer) (bFromSweep :type Boolean) (SweepResult :type Hit%20Result%20Structure%20%28by%20ref%29))
  (Utilities|Casting|CastToSideScrollerCharacter OtherActor)
  (Variables|Default|SetMove true)
  (Variables|Default|SetMoveReverse false))

(event OnComponentEndOverlap(Box)
  (params (OverlappedComponent :type Primitive%20Component%20Object%20Reference) (OtherActor :type Actor%20Object%20Reference) (OtherComp :type Primitive%20Component%20Object%20Reference) (OtherBodyIndex :type Integer))
  (Utilities|Casting|CastToSideScrollerCharacter OtherActor)
  (Variables|Default|SetMove false)
  (Variables|Default|SetMoveReverse true))

(event EventBeginPlay
  (Variables|Default|SetNegativeSpeed (* (Variables|Default|GetSpeed) -1.0)))

(event Collision|EventActorBeginOverlap
  (params (OtherActor :type Actor%20Object%20Reference)))

(event EventTick
  (params (DeltaSeconds :type Float%20%28single-precision%29))
  (if (Variables|Default|GetMove)
    (CallFunction|MoveonSpline (Variables|Default|GetSpeed))
    (elif (Variables|Default|GetMoveReverse)
      (CallFunction|MoveonSpline (Variables|Default|GetNegativeSpeed)))))

(fn ConstructionScript)

(fn MoveonSpline
  (params (Speed :type Float%20%28single-precision%29))
  (bind _spline (Variables|Default|GetSpline))
  (bind _output_get (Variables|Default|SetAmountToMove (* Speed (Utilities|Time|GetWorldDeltaSeconds))))
  (bind _output_get_2 (Variables|Default|SetDistanceAlongTheSpline (+ (Variables|Default|GetDistanceAlongTheSpline) _output_get)))
  (Transformation|SetWorldLocation (Variables|Default|GetCube) (Spline|GetLocationatDistanceAlongSpline _spline _output_get_2 "World") false false)
  (Utilities|FlowControl|Sequence
    (:then_0
      (if (<= (- (Spline|GetSplineLength _spline) (Variables|Default|GetDistanceAlongTheSpline)) 1.0)
        (Variables|Default|SetMove false)))
    (:then_1
      (if (<= (Variables|Default|GetDistanceAlongTheSpline) 1.0)
        (Variables|Default|SetMoveReverse false)))))