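; Moving enemy hazard for a side-scroller that sends the player back to their checkpoint on contact.
; While Move is set, Tick shifts the actor by Speed along the axis chosen by Direction, without sweep or delta-time scaling, so motion is frame-rate dependent and never reverses here.
; Overlap of any of its three cones by a SideScrollerCharacter calls RestartFromCheckPoint on player 0's character.
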(event OnComponentBeginOverlap(Cone)
  (params (OverlappedComponent :type Primitive%20Component%20Object%20Reference) (OtherActor :type Actor%20Object%20Reference) (OtherComp :type Primitive%20Component%20Object%20Reference) (OtherBodyIndex :type Integer) (bFromSweep :type Boolean) (SweepResult :type Hit%20Result%20Structure%20%28by%20ref%29))
  (Utilities|Casting|CastToSideScrollerCharacter OtherActor)
  (Game|GetCurrentLevelName true)
  (bind _asside_scroller_character (Utilities|Casting|CastToSideScrollerCharacter (Game|GetPlayerCharacter 0)))
  (Default|RestartfromCheckPoint _asside_scroller_character))

(event OnComponentBeginOverlap(Cone1)
  (params (OverlappedComponent :type Primitive%20Component%20Object%20Reference) (OtherActor :type Actor%20Object%20Reference) (OtherComp :type Primitive%20Component%20Object%20Reference) (OtherBodyIndex :type Integer) (bFromSweep :type Boolean) (SweepResult :type Hit%20Result%20Structure%20%28by%20ref%29))
  (Utilities|Casting|CastToSideScrollerCharacter OtherActor)
  (Game|GetCurrentLevelName true)
  (bind _asside_scroller_character (Utilities|Casting|CastToSideScrollerCharacter (Game|GetPlayerCharacter 0)))
  (Default|RestartfromCheckPoint _asside_scroller_character))

(event OnComponentBeginOverlap(Cone2)
  (params (OverlappedComponent :type Primitive%20Component%20Object%20Reference) (OtherActor :type Actor%20Object%20Reference) (OtherComp :type Primitive%20Component%20Object%20Reference) (OtherBodyIndex :type Integer) (bFromSweep :type Boolean) (SweepResult :type Hit%20Result%20Structure%20%28by%20ref%29))
  (Utilities|Casting|CastToSideScrollerCharacter OtherActor)
  (Game|GetCurrentLevelName true)
  (bind _asside_scroller_character (Utilities|Casting|CastToSideScrollerCharacter (Game|GetPlayerCharacter 0)))
  (Default|RestartfromCheckPoint _asside_scroller_character))

(event EventTick
  (params (DeltaSeconds :type Float%20%28single-precision%29))
  (bind _returnvalue (Transformation|GetActorLocation))
  (bind _speed (Variables|Default|GetSpeed))
  (if (Variables|Default|Getmove)
    (switch string (Variables|Default|GetDirection)
      (:x
        (Variables|Default|Setvelocity (Math|Vector|MakeVector (+ (.x _returnvalue) (Variables|Default|GetSpeed)) (.y _returnvalue) (.z _returnvalue))))
      (:y
        (Variables|Default|Setvelocity (Math|Vector|MakeVector (.x _returnvalue) (+ (.y _returnvalue) _speed) (.z _returnvalue))))
      (:z
        (Variables|Default|Setvelocity (Math|Vector|MakeVector (.x _returnvalue) (.y _returnvalue) (+ _speed (.z _returnvalue))))))
    (Transformation|SetActorLocation (Variables|Default|Getvelocity) false false)))

(fn ConstructionScript)