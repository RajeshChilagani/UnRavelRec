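; MovingPlatform_Con is a moving platform that travels back and forth along one world axis.
; BeginPlay stores the start location and offsets it by DistanceToMove on the X, Y or Z axis chosen by Direction to get the end point.
; Tick plays or reverses a timeline according to PlayFromReverse; the timeline lerps the actor between both points and flips that flag on finishing.
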(event EventBeginPlay
  (bind _returnvalue (Transformation|GetActorLocation))
  (bind _returnvalue_2 (Transformation|GetActorLocation))
  (bind _returnvalue_3 (Transformation|GetActorLocation))
  (Variables|Default|SetStartPoint (Transformation|GetActorLocation))
  (switch int (Variables|Default|GetDirection)
    (:1
      (Variables|Default|SetEndPoint (Math|Vector|MakeVector (+ (Variables|Default|GetDistanceToMove) (.x _returnvalue)) (.y _returnvalue) (.z _returnvalue))))
    (:2
      (Variables|Default|SetEndPoint (Math|Vector|MakeVector (.x _returnvalue_2) (+ (Variables|Default|GetDistanceToMove) (.y _returnvalue_2)) (.z _returnvalue_2))))
    (:3
      (Variables|Default|SetEndPoint (Math|Vector|MakeVector (.x _returnvalue_3) (.y _returnvalue_3) (+ (Variables|Default|GetDistanceToMove) (.z _returnvalue_3)))))))

(event Collision|EventActorBeginOverlap
  (params (OtherActor :type Actor%20Object%20Reference)))

(event EventTick
  (params (DeltaSeconds :type Float%20%28single-precision%29))
  (if (Variables|Default|GetPlayFromReverse)
    (bind _newtrack_0 (Timeline|Timeline_0 Reverse)
      (:Update
        (Transformation|SetActorLocation (Math|Vector|Lerp(Vector) (Variables|Default|GetStartPoint) (Variables|Default|GetEndPoint) _newtrack_0) false false))
      (:Finished
        (if (Variables|Default|GetPlayFromReverse)
          (Variables|Default|SetPlayFromReverse false)
          (else
            (Variables|Default|SetPlayFromReverse true)))))
    (else
      (Timeline|Timeline_0 Play))))

(fn ConstructionScript)