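; EnemyInstigator is a spawner actor that starts producing moving enemies once the side-scroller character overlaps its Trigger component.
; The overlap sets StartSpawning, which is never cleared, and a Delay on Tick paces spawns to roughly every two seconds.
; Each EnemeymovingNoTrigger spawns at the actor's transform with a random vertical offset, then is set moving along "y" at a fixed speed.
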(event OnComponentBeginOverlap(Trigger)
  (params (OverlappedComponent :type Primitive%20Component%20Object%20Reference) (OtherActor :type Actor%20Object%20Reference) (OtherComp :type Primitive%20Component%20Object%20Reference) (OtherBodyIndex :type Integer) (bFromSweep :type Boolean) (SweepResult :type Hit%20Result%20Structure%20%28by%20ref%29))
  (Utilities|Casting|CastToSideScrollerCharacter OtherActor)
  (Variables|Default|SetStartSpawning true))

(event EventTick
  (params (DeltaSeconds :type Float%20%28single-precision%29))
  (bind _returnvalue (Transformation|GetActorTransform))
  (if (Variables|Default|GetStartSpawning)
    (Utilities|FlowControl|Sequence
      (:then_0
        (Utilities|FlowControl|Delay 2.0)
        (bind _returnvalue_2 (Game|SpawnActorfromClass "/Game/Blueprints/enemeymovingNoTrigger.enemeymovingNoTrigger_C" (Math|Transform|MakeTransform (Math|Vector|MakeVector (.x (.location _returnvalue)) (.y (.location _returnvalue)) (+ (.z (.location _returnvalue)) (Math|Random|RandomFloatinRange -6e+02 6e+02))) (.rotation _returnvalue) (.scale _returnvalue)) "AlwaysSpawn" 0 0))
        (Variables|/Game/Blueprints/enemeymovingNoTrigger.enemeymovingNoTrigger_C|SetDirection _returnvalue_2 "y")
        (Variables|/Game/Blueprints/enemeymovingNoTrigger.enemeymovingNoTrigger_C|SetSpeed _returnvalue_2 5.0)
        (Variables|/Game/Blueprints/enemeymovingNoTrigger.enemeymovingNoTrigger_C|Setmove _returnvalue_2 true)))))

(fn ConstructionScript)